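; Deprecated projectile Blueprint that flies on a set path, then homes in on a referenced character.
; Until a gate closes, Tick sets local-space velocity from a stored vector with a sideways offset and accumulates elapsed time.
; After about three seconds, the gate stops that steering and a DoOnce enables ProjectileMovement homing on the character's capsule, sets max speed and prints the target's name.
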(event EventBeginPlay)

(event EventTick
  (params (DeltaSeconds :type Float%20%28single-precision%29))
  (bind _velo (Variables|Default|GetVelo))
  (bind _projectilemovement (Variables|Default|GetProjectileMovement))
  (if (not (Variables|Default|GetGate))
    (Game|Components|ProjectileMovement|SetVelocityinLocalSpace (Variables|Default|GetProjectileMovement) (Math|Vector|MakeVector (.x _velo) (+ (.y _velo) 2e+01) 0.0))
    (bind _output_get (Variables|Default|SetSec (+ (Variables|Default|GetSec) DeltaSeconds)))
    (Variables|Default|SetGate (>= _output_get 3.2))
    (if (>= _output_get 3.2)
      (Utilities|FlowControl|DoOnce false
        (:Completed
          (Variables|/Script/Engine.ProjectileMovementComponent|SetbIsHomingProjectile (Variables|Default|GetProjectileMovement) true)
          (Variables|/Script/Engine.ProjectileMovementComponent|SetMaxSpeed _projectilemovement 2.5e+03)
          (bind _output_get_2 (Variables|/Script/Engine.ProjectileMovementComponent|SetHomingTargetComponent _projectilemovement (Variables|/Script/Engine.Character|GetCapsuleComponent (Variables|Default|GetCharRef))))
          (Development|PrintString (Utilities|GetObjectName _output_get_2)))))))

(fn ConstructionScript)