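; Thrown boomerang actor, in a Deprecated folder, that flies out, returns to its instigator and is caught by BP_FPSCharacter on overlap.
; Chained timelines drive the Sphere forward, backward if the thrower is far, then lerp it home, accelerating up close, while a timer spins the mesh.
; Sphere hits stop flight and drop the mesh with physics; mesh hits resync the Sphere for pickup.
; Destruction triggers the thrower's camera shake.
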(event OnComponentHit(Sphere)
  (params (HitComponent :type Primitive%20Component%20Object%20Reference) (OtherActor :type Actor%20Object%20Reference) (OtherComp :type Primitive%20Component%20Object%20Reference) (NormalImpulse :type Vector :default "0, 0, 0") (Hit :type Hit%20Result%20Structure%20%28by%20ref%29))
  (bind _staticmesh (Variables|Default|GetStaticMesh))
  ;[1 1 1] When boomerang hit stop timeline, clear timer, ticking disabled. Simulate physics is activated!
  (Components|Activation|Deactivate (Variables|Default|GetToTheCharacter))
  (Components|Activation|Deactivate (Variables|Default|GetForward))
  (Components|Activation|Deactivate (Variables|Default|GetBackward))
  (Utilities|Time|ClearandInvalidateTimerbyHandle (Variables|Default|GetRotateTimerHandle))
  (Actor|Tick|SetActorTickEnabled false)
  (Collision|SetCollisionResponsetoAllChannels _staticmesh "ECR_Block")
  (Collision|SetCollisionEnabled (Variables|Default|GetStaticMesh) "PhysicsOnly")
  (Collision|SetCollisionResponsetoChannel (Variables|Default|GetSphere) "ECC_Pawn" "ECR_Overlap")
  (Physics|SetSimulatePhysics _staticmesh true))

(event OnComponentHit(StaticMesh)
  (params (HitComponent :type Primitive%20Component%20Object%20Reference) (OtherActor :type Actor%20Object%20Reference) (OtherComp :type Primitive%20Component%20Object%20Reference) (NormalImpulse :type Vector :default "0, 0, 0") (Hit :type Hit%20Result%20Structure%20%28by%20ref%29))
  ;[1 1 1] When Sphere hit wall or etc. static mesh falls correctly but sphere location stops hit location. So when mesh hit, sphere's location is updated
  (Transformation|SetWorldLocation (Variables|Default|GetSphere) (Transformation|GetWorldLocation (Variables|Default|GetStaticMesh)) false true))

(event OnComponentBeginOverlap(Sphere)
  (params (OverlappedComponent :type Primitive%20Component%20Object%20Reference) (OtherActor :type Actor%20Object%20Reference) (OtherComp :type Primitive%20Component%20Object%20Reference) (OtherBodyIndex :type Integer) (bFromSweep :type Boolean) (SweepResult :type Hit%20Result%20Structure%20%28by%20ref%29))
  ;[1 1 1] To get boomerang
  (bind _asbp_fpscharacter (Utilities|Casting|CastToBP_FPSCharacter OtherActor))
  (Default|TakeBoomerang _asbp_fpscharacter)
  (Utilities|FlowControl|Delay 0.0)
  (Actor|DestroyActor))

(event Custom|RotateMesh
  ;[1 1 1] While moving boomerang rotates
  (Transformation|AddLocalRotation (Variables|Default|GetStaticMesh) "0,6.000000, 0" false false))

(event EventDestroyed
  (bind _asbp_fpscharacter (Utilities|Casting|CastToBP_FPSCharacter (Variables|Default|GetInstigatorPawnRef)))
  (Default|BoomerangCamShake _asbp_fpscharacter))

(event EventBeginPlay
  (bind _tothecharacter (Variables|Default|GetToTheCharacter))
  ;[1 1 1] To turn back character, get reference of pawn
  (Variables|Default|SetInstigatorPawnRef (Game|GetInstigator))
  ;[1 1 1] to prevent pawn = nullptr
  (Utilities|FlowControl|Delay 0.0)
  (Actor|Tick|SetActorTickEnabled false)
  (bind _returnvalue (Utilities|Time|SetTimerbyEvent (delegate Custom|RotateMesh) (Utilities|Time|GetWorldDeltaSeconds) true))
  (Variables|Default|SetRotateTimerHandle _returnvalue)
  (Variables|Default|SetInitialLocation (Transformation|GetActorLocation))
  (Components|Timeline|SetPlayRate (Variables|Default|GetForward) (Variables|Default|GetTimelineRate))
  (bind _deltalocation (Timeline|Forward PlayFromStart)
    (:Update
      (Transformation|AddLocalOffset (Variables|Default|GetSphere) (* _deltalocation (Variables|Default|GetBoomerangRangeMultiplier)) true false))
    (:Finished
      (Variables|Default|SetReturnStartLocation (Transformation|GetWorldLocation (Variables|Default|GetSphere)))
      (Components|Timeline|SetPlayRate (Variables|Default|GetBackward) (+ (Variables|Default|GetTimelineRate) 0.0))
      (if (>= (Math|Vector|Distance(Vector) (Transformation|GetWorldLocation (Variables|Default|GetSphere)) (Transformation|GetActorLocation (Variables|Default|GetInstigatorPawnRef))) 7e+02)
        (bind _deltalocation_2 (Timeline|Backward PlayFromStart)
          (:Update
            (Transformation|AddLocalOffset (Variables|Default|GetSphere) (* _deltalocation_2 (Variables|Default|GetBoomerangRangeMultiplier)) true false))
          (:Finished
            (Variables|Default|SetReturnStartLocation (Transformation|GetWorldLocation (Variables|Default|GetSphere)) :!label _label)
            (Components|Timeline|SetPlayRate (Variables|Default|GetToTheCharacter) (Variables|Default|GetTimelineRate))
            (bind _alpha (Timeline|ToTheCharacter PlayFromStart)
              (:Update
                (if (<= (Math|Vector|Distance(Vector) (Transformation|GetWorldLocation (Variables|Default|GetSphere)) (Transformation|GetActorLocation (Variables|Default|GetInstigatorPawnRef))) 2e+02)
                  (Components|Timeline|SetPlayRate _tothecharacter (+ (Components|Animation|GetPlayRate _tothecharacter) _alpha)))
                (Transformation|SetWorldLocation (Variables|Default|GetSphere) (Math|Vector|Lerp(Vector) (Variables|Default|GetReturnStartLocation) (Transformation|GetActorLocation (Variables|Default|GetInstigatorPawnRef)) _alpha) true false)))))
        (else
          (goto _label))))))

(event EventTick
  (params (DeltaSeconds :type Float%20%28single-precision%29))
  ;[1 1 1] Turn back while ticking. Initially is not ticking!
  (Transformation|SetActorLocation (Math|Interpolation|VInterpTo (Transformation|GetActorLocation) (Transformation|GetActorLocation (Variables|Default|GetInstigatorPawnRef)) DeltaSeconds 1e+01) true false))

(fn ConstructionScript
  (Actor|Tick|SetActorTickEnabled false))