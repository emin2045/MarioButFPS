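; BP_SaveGameTrigger is a one-shot checkpoint volume that records the player's respawn point.
; When an actor tagged "Us" enters its box, it converts the SpawnLocation offset to world space and sends it to the GameInstance as the current spawn point.
; It then shows the WBP_Saved widget, destroys itself and plays the Prize sound.
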(event OnComponentBeginOverlap(Box)
  (params (OverlappedComponent :type Primitive%20Component%20Object%20Reference) (OtherActor :type Actor%20Object%20Reference) (OtherComp :type Primitive%20Component%20Object%20Reference) (OtherBodyIndex :type Integer) (bFromSweep :type Boolean) (SweepResult :type Hit%20Result%20Structure%20%28by%20ref%29))
  (if (Actor|ActorHasTag OtherActor "Us")
    (Class|BPISaveSystem|SetCurrentSpawnPoint(Message) (Game|GetGameInstance) (Math|Transform|TransformLocation (Transformation|GetActorTransform) (Variables|Default|GetSpawnLocation)))
    (bind _returnvalue (UserInterface|CreateWidget "/Game/Blueprints/Character/WBP_Saved.WBP_Saved_C"))
    (UserInterface|Viewport|AddtoViewport _returnvalue 0)
    (Actor|DestroyActor)
    (Audio|PlaySound2D "/Game/Sounds/Gameplay/prize.prize" 1.0 1.0 0.0 0 0)))

(fn ConstructionScript)