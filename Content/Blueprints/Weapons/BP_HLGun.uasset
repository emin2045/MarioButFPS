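; BP_HLGun is a weapon pickup that grants the player use of the HL gun.
; When an actor tagged "Us" overlaps its sphere, it sends that actor TakeHLGunMessage, destroys itself and plays a prize sound.
; The construction script gives the skeletal mesh's two material slots dynamic instances tinted bright orange.
; An OutputTry function is a stub that always returns false.
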(event OnComponentBeginOverlap(Sphere)
  (params (OverlappedComponent :type Primitive%20Component%20Object%20Reference) (OtherActor :type Actor%20Object%20Reference) (OtherComp :type Primitive%20Component%20Object%20Reference) (OtherBodyIndex :type Integer) (bFromSweep :type Boolean) (SweepResult :type Hit%20Result%20Structure%20%28by%20ref%29))
  (if (Actor|ActorHasTag OtherActor "Us")
    (Class|BPIInteraction|TakeHLGun(Message) OtherActor)
    (Actor|DestroyActor)
    (Audio|PlaySound2D "/Game/Sounds/Gameplay/prize.prize" 1.0 1.0 0.0 0 0)))

(event EventBeginPlay)

(event Collision|EventActorBeginOverlap
  (params (OtherActor :type Actor%20Object%20Reference)))

(event EventTick
  (params (DeltaSeconds :type Float%20%28single-precision%29)))

(fn ConstructionScript
  (bind _skeletalmesh (Variables|Default|GetSkeletalMesh))
  (bind _returnvalue (Rendering|Material|CreateDynamicMaterialInstance _skeletalmesh 1 0 "None" :!class /Script/Engine.PrimitiveComponent))
  (Rendering|Material|SetVectorParameterValue _returnvalue "Color" "(R=10.000000,G=3.254032,B=0.216648,A=1.000000)" :!class /Script/Engine.MaterialInstanceDynamic)
  (bind _returnvalue_2 (Rendering|Material|CreateDynamicMaterialInstance _skeletalmesh 0 0 "None" :!class /Script/Engine.PrimitiveComponent))
  (Rendering|Material|SetVectorParameterValue _returnvalue_2 "Color" "(R=10.000000,G=2.095414,B=0.091017,A=1.000000)" :!class /Script/Engine.MaterialInstanceDynamic))

(fn OutputTry
  (params (Input :type Integer))
  (return false))