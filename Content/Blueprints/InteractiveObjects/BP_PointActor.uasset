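; A scoring target that awards a point when an actor tagged PointObject overlaps its sphere.
; On overlap it swaps the mesh material, calls MadeScoreMessage on the point manager, plays a coin sound and gives both actors a short lifespan.
; A looping timer, set to the current frame delta, lifts the actor cosmetically until it expires.
; Nothing guards against repeated overlaps during that lifespan, and OutputTry is a stub returning false.
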(event OnComponentBeginOverlap(Sphere)
  (params (OverlappedComponent :type Primitive%20Component%20Object%20Reference) (OtherActor :type Actor%20Object%20Reference) (OtherComp :type Primitive%20Component%20Object%20Reference) (OtherBodyIndex :type Integer) (bFromSweep :type Boolean) (SweepResult :type Hit%20Result%20Structure%20%28by%20ref%29))
  (if (Actor|ActorHasTag OtherActor "PointObject")
    (Rendering|Material|SetMaterial (Variables|Default|GetStaticMesh) 0 "/Engine/MapTemplates/Materials/BasicAsset03.BasicAsset03")
    (Actor|SetLifeSpan OtherActor 3.0)
    (Actor|SetLifeSpan 3.0)
    (Class|BPIInteraction|MadeScore(Message) (Variables|Default|GetPointManagerRef))
    (Utilities|Time|SetTimerbyEvent (delegate Custom|RaiseObject) (Utilities|Time|GetWorldDeltaSeconds) true)
    (Audio|PlaySound2D "/Game/Sounds/Gameplay/coin_sound.coin_sound" 1.0 1.0 0.0 0 0)))

(event Custom|RaiseObject
  ;[1 1 1] this is for cosmetic, just raise the actor
  (Transformation|AddWorldOffset (Variables|Default|GetDefaultSceneRoot) "0, 0,10.000000" true false))

(fn ConstructionScript)

(fn OutputTry
  (params (Input :type Integer))
  (return false))