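; Draggable actor that a nearby BP_FPSCharacter can push, pull or slide sideways while holding the push key.
; Box overlaps store the character reference and toggle Tick, which plays a sound every frame the key is held.
; Tick applies swept local offsets along the mesh's hit normal from forward input, or swaps its X/Y for sideways input, which takes priority.
; OutputTry is a stub returning false.
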(event OnComponentHit(MeshToGrab)
  (params (HitComponent :type Primitive%20Component%20Object%20Reference) (OtherActor :type Actor%20Object%20Reference) (OtherComp :type Primitive%20Component%20Object%20Reference) (NormalImpulse :type Vector :default "0, 0, 0") (Hit :type Hit%20Result%20Structure%20%28by%20ref%29)))

(event OnComponentBeginOverlap(Box)
  (params (OverlappedComponent :type Primitive%20Component%20Object%20Reference) (OtherActor :type Actor%20Object%20Reference) (OtherComp :type Primitive%20Component%20Object%20Reference) (OtherBodyIndex :type Integer) (bFromSweep :type Boolean) (SweepResult :type Hit%20Result%20Structure%20%28by%20ref%29))
  ;[1 1 1] Character is near enough
  (bind _asbp_fpscharacter (Utilities|Casting|CastToBP_FPSCharacter OtherActor))
  (Variables|Default|SetCharRef _asbp_fpscharacter)
  (Actor|Tick|SetActorTickEnabled true))

(event OnComponentEndOverlap(Box)
  (params (OverlappedComponent :type Primitive%20Component%20Object%20Reference) (OtherActor :type Actor%20Object%20Reference) (OtherComp :type Primitive%20Component%20Object%20Reference) (OtherBodyIndex :type Integer))
  ;[1 1 1] Character is not near enough
  (if (== OtherActor (Variables|Default|GetCharRef))
    (Variables|Default|SetCharRef (Variables|Default|GetNullptr))
    (Actor|Tick|SetActorTickEnabled false)))

(event EventTick
  (params (DeltaSeconds :type Float%20%28single-precision%29))
  (bind _charref (Variables|Default|GetCharRef)
    (:then
      (if (Variables|/Game/Blueprints/Character/BP_FPSCharacter.BP_FPSCharacter_C|GetbPushKeyDown _charref) ; Is character pressing push button
        (Audio|SpawnSound2D "/Game/Sounds/Swings/AxeSwing3.AxeSwing3" 0.4 1.5 0.0 0)
        (if (== (Variables|/Game/Blueprints/Character/BP_FPSCharacter.BP_FPSCharacter_C|GetMoveRightAxisValue (Variables|Default|GetCharRef)) 0.0) ; pressing right button?
          (Transformation|AddActorLocalOffset (* (* (* (.impactnormal (stale OnComponentHit(MeshToGrab) Hit)) 1.5e+02) DeltaSeconds) (Variables|/Game/Blueprints/Character/BP_FPSCharacter.BP_FPSCharacter_C|GetMoveForwardAxisValue (Variables|Default|GetCharRef))) true false) ; if forward axis value is negative, it pulls if not it pushes
          (elif (!= (.Y (Math|Vector|BreakVector (.impactnormal (stale OnComponentHit(MeshToGrab) Hit)))) 0.0) ; if true pin executes, drag object to left, Otherwise drag object to right
            (Transformation|AddActorLocalOffset (* (Math|Vector|MakeVector (.Y (Math|Vector|BreakVector (* (* (.impactnormal (stale OnComponentHit(MeshToGrab) Hit)) 1.5e+02) DeltaSeconds))) (.X (Math|Vector|BreakVector (* (* (.impactnormal (stale OnComponentHit(MeshToGrab) Hit)) 1.5e+02) DeltaSeconds))) (.Z (Math|Vector|BreakVector (* (* (.impactnormal (stale OnComponentHit(MeshToGrab) Hit)) 1.5e+02) DeltaSeconds)))) (* (Variables|/Game/Blueprints/Character/BP_FPSCharacter.BP_FPSCharacter_C|GetMoveRightAxisValue (Variables|Default|GetCharRef)) -1.0)) true false)
            (else
              (Transformation|AddActorLocalOffset (* (Math|Vector|MakeVector (.Y (Math|Vector|BreakVector (* (* (.impactnormal (stale OnComponentHit(MeshToGrab) Hit)) 1.5e+02) DeltaSeconds))) (.X (Math|Vector|BreakVector (* (* (.impactnormal (stale OnComponentHit(MeshToGrab) Hit)) 1.5e+02) DeltaSeconds))) (.Z (Math|Vector|BreakVector (* (* (.impactnormal (stale OnComponentHit(MeshToGrab) Hit)) 1.5e+02) DeltaSeconds)))) (Variables|/Game/Blueprints/Character/BP_FPSCharacter.BP_FPSCharacter_C|GetMoveRightAxisValue (Variables|Default|GetCharRef))) true false))))))
    (:else)))

(fn ConstructionScript)

(fn OutputTry
  (params (Input :type Integer))
  (return false))