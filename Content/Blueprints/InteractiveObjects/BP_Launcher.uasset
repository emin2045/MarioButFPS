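; BP_Launcher is a launch pad that propels any Character overlapping its Box and plays a metal jump-land foley sound in 2D.
; An airborne character is launched straight up, while a grounded one is launched along its forward vector plus the Direction variable, both scaled by LaunchStrength.
; Both launches override the character's existing XY and Z velocity.
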(event OnComponentBeginOverlap(Box)
  (params (OverlappedComponent :type Primitive%20Component%20Object%20Reference) (OtherActor :type Actor%20Object%20Reference) (OtherComp :type Primitive%20Component%20Object%20Reference) (OtherBodyIndex :type Integer) (bFromSweep :type Boolean) (SweepResult :type Hit%20Result%20Structure%20%28by%20ref%29))
  (bind _ascharacter (Utilities|Casting|CastToCharacter OtherActor))
  (Audio|SpawnSound2D "/Game/Sounds/FootstepJump/sw_Foley_JumpLand_Metal_03.sw_Foley_JumpLand_Metal_03" 1.0 1.0 0.0 0)
  (if (AI|Components|NavMovement|IsFalling (Variables|/Script/Engine.Character|GetCharacterMovement _ascharacter)) ; is in air
    (Character|LaunchCharacter _ascharacter (* (Math|Vector|VectorUp) (Variables|Default|GetLaunchStrength)) true true)
    (else
      (Character|LaunchCharacter _ascharacter (* (+ (Transformation|GetActorForwardVector _ascharacter) (Variables|Default|GetDirection)) (Variables|Default|GetLaunchStrength)) true true))))

(fn ConstructionScript)