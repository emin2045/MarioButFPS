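; BP_MissionDoor is an interactive door that a nearby actor tagged "Us" enables for opening with the OpenDoor input.
; Box overlap events toggle the CanOpenDoor flag and show or hide a TextRender.
; Pressing OpenDoor while enabled destroys both the box and text, plays a 2D sound, and runs a Timeline that swings the whole actor to -90 degrees yaw.
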(event OnComponentBeginOverlap(Box)
  (params (OverlappedComponent :type Primitive%20Component%20Object%20Reference) (OtherActor :type Actor%20Object%20Reference) (OtherComp :type Primitive%20Component%20Object%20Reference) (OtherBodyIndex :type Integer) (bFromSweep :type Boolean) (SweepResult :type Hit%20Result%20Structure%20%28by%20ref%29))
  (if (Actor|ActorHasTag OtherActor "Us")
    (Variables|Default|SetbCanOpenDoor true)
    (Rendering|SetVisibility (Variables|Default|GetTextRender) true false)))

(event OnComponentEndOverlap(Box)
  (params (OverlappedComponent :type Primitive%20Component%20Object%20Reference) (OtherActor :type Actor%20Object%20Reference) (OtherComp :type Primitive%20Component%20Object%20Reference) (OtherBodyIndex :type Integer))
  (if (Actor|ActorHasTag OtherActor "Us")
    (Variables|Default|SetbCanOpenDoor false)
    (Rendering|SetVisibility (Variables|Default|GetTextRender) false false)))

(event Input|ActionEvents|InputActionOpenDoor
  (params (Key :type Key%20Structure))
  (:Pressed
    (if (Variables|Default|GetbCanOpenDoor)
      (Components|DestroyComponent (Variables|Default|GetBox))
      (Audio|SpawnSound2D "/Engine/VREditor/Sounds/UI/Floating_UI_Open-002.Floating_UI_Open-002" 1.0 1.0 0.0 0)
      (bind _alpha (Timeline|Timeline_0 PlayFromStart)
        (:Update
          (Transformation|SetActorRelativeRotation (Math|Rotator|MakeRotator 0.0 0.0 (Math|Float|Lerp 0.0 -9e+01 _alpha))))))))

(fn ConstructionScript)