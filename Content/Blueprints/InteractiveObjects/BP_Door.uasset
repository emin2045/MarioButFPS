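; An interactive door actor that swings open once when a player presses the OpenDoor input nearby.
; A box trigger detects actors tagged "Us", enabling the input and showing a text prompt.
; Opening removes the trigger and prompt, then a timeline lerps the actor's yaw to a quarter turn.
; On BeginPlay it binds to a character's ShowYourselfDoors event, printing the message and its name once before unbinding.
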(event OnComponentBeginOverlap(Box)
  (params (OverlappedComponent :type Primitive%20Component%20Object%20Reference) (OtherActor :type Actor%20Object%20Reference) (OtherComp :type Primitive%20Component%20Object%20Reference) (OtherBodyIndex :type Integer) (bFromSweep :type Boolean) (SweepResult :type Hit%20Result%20Structure%20%28by%20ref%29))
  (if (Actor|ActorHasTag OtherActor "Us")
    (Variables|Default|SetbCanOpenDoor true)
    (Rendering|SetVisibility (Variables|Default|GetTextRender) true false)))

(event OnComponentEndOverlap(Box)
  (params (OverlappedComponent :type Primitive%20Component%20Object%20Reference) (OtherActor :type Actor%20Object%20Reference) (OtherComp :type Primitive%20Component%20Object%20Reference) (OtherBodyIndex :type Integer))
  (if (Actor|ActorHasTag OtherActor "Us")
    (Variables|Default|SetbCanOpenDoor false)
    (Rendering|SetVisibility (Variables|Default|GetTextRender) false false)))

(event Custom|ZAAAA
  (params (Message :type Name))
  (Development|PrintString (Utilities|String|Append (Utilities|String|ToString(Name) Message) ":::" (Utilities|GetObjectName self)))
  (EventDispatchers|UnbindEventfromShowYourselfDoors (Variables|Default|GetCharRef) (delegate Custom|ZAAAA)))

(event EventBeginPlay
  (EventDispatchers|BindEventtoShowYourselfDoors (Variables|Default|GetCharRef) (delegate Custom|ZAAAA)))

(event Input|ActionEvents|InputActionOpenDoor
  (params (Key :type Key%20Structure :default "None"))
  (:Pressed
    (if (Variables|Default|GetbCanOpenDoor)
      (Components|DestroyComponent (Variables|Default|GetBox))
      (bind _newtrack_0 (Timeline|Timeline_0 PlayFromStart)
        (:Update
          (Transformation|SetActorRotation (Math|Rotator|MakeRotator 0.0 0.0 (Math|Float|Lerp 0.0 -9e+01 _newtrack_0))))))))

(fn ConstructionScript)

(fn OutputTry
  (params (Input :type Integer))
  (return false))