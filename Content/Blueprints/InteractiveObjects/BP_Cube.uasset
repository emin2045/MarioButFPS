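; BP_Cube is an interactive physics cube that the character can release with a push and knock around with weapon fire.
; FallingStart, called from BP_Character, enables physics on MeshToGrab, applies a directional impulse with extra lift when jumping, and restores blocking against pawns and physics bodies.
; AddImpulsetoObject pushes the hit component at the impact point with a clamped force that grows per hit and resets through a retriggerable delay once hits stop.
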(event Custom|FallingStart
  (params (Direction :type Vector) (bJump :type Boolean) (ImpulseAmount :type Float%20%28single-precision%29))
  (bind _returnvalue (* Direction ImpulseAmount))
  ;[1 1 1] Called from BP_Character
  (if bJump
    (Variables|Default|SetJumpFactor (Variables|Default|GetMaxJumpFactor))
    (else
      (Variables|Default|SetJumpFactor 0.0)))
  (Physics|SetSimulatePhysics (Variables|Default|GetMeshToGrab) true)
  (Physics|AddImpulse (Variables|Default|GetMeshToGrab) (Math|Vector|MakeVector (.x _returnvalue) (.y _returnvalue) (+ (.z _returnvalue) (Variables|Default|GetJumpFactor))) "None" false)
  (Collision|SetCollisionResponsetoChannel (Variables|Default|GetMeshToGrab) "ECC_Pawn" "ECR_Block")
  (Collision|SetCollisionResponsetoChannel (Variables|Default|GetMeshToGrab) "ECC_PhysicsBody" "ECR_Block"))

(event EventAddImpulsetoObject
  (params (HitComp :type Primitive%20Component%20Object%20Reference) (ImpactPoint :type Vector :default "0, 0, 0") (OtherActorForwardVector :type Vector :default "0, 0, 0"))
  ;[1 1 1] When this actor hit by character with a weapon, its called from character
  (bind _output_get (Variables|Default|SetMachineGunForceAmount (Math|Float|Clamp(Float) (+ (Variables|Default|GetMachineGunForceAmount) 7.5e+02) 5e+03 3.5e+04)))
  (Physics|AddImpulseatLocation HitComp (* OtherActorForwardVector _output_get) ImpactPoint "None")
  (Utilities|FlowControl|RetriggerableDelay 2.0)
  (Variables|Default|SetMachineGunForceAmount 5e+03))

(fn ConstructionScript)

(fn OutputTry
  (params (Input :type Integer))
  (return false))