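; Black hole actor that affects physics objects, the player and enemies overlapping its sphere, centered on a point raised above it.
; Each tick, it applies mass-scaled radial force to components tagged PhysicObject.
; It triggers BlackholeImpact once on the player, found by capsule tag, and calls BlackholeEffect on overlapping enemies each tick.
; On destruction, it clears the affected player's black hole flag and restores walking movement.
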(event EventDestroyed
  ;[1 1 1] When this actor destroyed, it cause to stop applying force to Character
  (bind _charref (Variables|Default|GetCharRef)
    (:then
      (Variables|/Game/Blueprints/Character/BP_FPSCharacter.BP_FPSCharacter_C|SetbBlackholeActivated _charref false)
      (Pawn|Components|CharacterMovement|SetMovementMode (Variables|/Script/Engine.Character|GetCharacterMovement _charref) "MOVE_Walking" 0))
    (:else)))

(event EventTick
  (params (DeltaSeconds :type Float%20%28single-precision%29))
  (bind _returnvalue (Transformation|GetActorLocation))
  (bind _sphere (Variables|Default|GetSphere))
  (bind _sphere_2 (Variables|Default|GetSphere))
  (bind _returnvalue_2 (Transformation|GetWorldLocation _sphere))
  (bind _returnvalue_3 (Transformation|GetWorldLocation _sphere_2))
  (for _array_element (Class|PrimitiveComponent|GetOverlappingComponents (Variables|Default|GetSphere))
    (if (Components|ComponentHasTag _array_element "PhysicObject")
      ;[1 1 1] If overlapped actor is cube or pychisc active object apply force
      (Physics|AddRadialForce _array_element (Math|Vector|MakeVector (.x _returnvalue) (.y _returnvalue) (+ (.z _returnvalue) 2e+02)) (Variables|/Script/Engine.SphereComponent|GetSphereRadius (Variables|Default|GetSphere)) (+ (* (Physics|GetMass _array_element) 6.0) (Variables|Default|GetDefaultStrength)) "RIF_Constant" true)
      (elif (Components|ComponentHasTag _array_element "CharCapsule")
        ;[1 1 1] If overlapped actor is the player
        (bind _asbp_fpscharacter (Utilities|Casting|CastToBP_FPSCharacter (Components|GetOwner _array_element))
          (:then
            (bind _output_get (Variables|Default|SetCharRef _asbp_fpscharacter))
            (Utilities|FlowControl|DoOnce false
              (:Completed
                (Default|BlackholeImpact _output_get (Math|Vector|MakeVector (.x _returnvalue_3) (.y _returnvalue_3) (+ (.z _returnvalue_3) 2e+02))))))
          (:CastFailed
            ;[1 1 1] If overlapped actor is enemy
            (bind _asbp_enemy_ai (Utilities|Casting|CastToBP_EnemyAI (Components|GetOwner _array_element)))
            (Default|BlackholeEffect _asbp_enemy_ai (Math|Vector|MakeVector (.x _returnvalue_2) (.y _returnvalue_2) (+ (.z _returnvalue_2) 2e+02)))))))))

(fn ConstructionScript)