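; Deprecated boomerang projectile that BP_FPSCharacter throws, calls back and catches.
; A Forward timeline moves the spinning boomerang along a charge-scaled path, switching to Tick homing if near the thrower at the distance check.
; Hits or timeline end drop the mesh into physics; once landed, CallBackBoomerang lifts it and lerps it back at a distance-scaled play rate.
; Character overlap triggers TakeBoomerang and destroys it, firing the character's camera shake.
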(event OnComponentHit(Sphere)
  (params (HitComponent :type Primitive%20Component%20Object%20Reference) (OtherActor :type Actor%20Object%20Reference) (OtherComp :type Primitive%20Component%20Object%20Reference) (NormalImpulse :type Vector :default "0, 0, 0") (Hit :type Hit%20Result%20Structure%20%28by%20ref%29))
  (bind _staticmesh (Variables|Default|GetStaticMesh))
  ;[1 1 1] When boomerang hit stop timeline, clear timer, ticking disabled. Simulate physics is activated!
  (Components|Activation|Deactivate (Variables|Default|GetForward))
  (Utilities|Time|PauseTimerbyHandle (Variables|Default|GetRotateTimerHandle))
  (Actor|Tick|SetActorTickEnabled false)
  (Collision|SetCollisionResponsetoAllChannels _staticmesh "ECR_Block")
  (Collision|SetCollisionEnabled (Variables|Default|GetStaticMesh) "PhysicsOnly")
  (Collision|SetCollisionResponsetoChannel (Variables|Default|GetSphere) "ECC_Pawn" "ECR_Overlap")
  (Physics|SetSimulatePhysics _staticmesh true))

(event OnComponentHit(StaticMesh)
  (params (HitComponent :type Primitive%20Component%20Object%20Reference) (OtherActor :type Actor%20Object%20Reference) (OtherComp :type Primitive%20Component%20Object%20Reference) (NormalImpulse :type Vector :default "0, 0, 0") (Hit :type Hit%20Result%20Structure%20%28by%20ref%29))
  ;[1 1 1] When Sphere hit wall or etc. static mesh falls correctly but sphere location stops hit location. So when mesh hit, sphere's location is updated
  (if (not (Variables|Default|GetbCalled))
    (Transformation|SetWorldLocation (Variables|Default|GetSphere) (Transformation|GetWorldLocation (Variables|Default|GetStaticMesh)) false true)
    (bind _result (Math|Integer|IncrementInt (Variables|Default|GetbHitFirst))
      (:%20%20
        (if (> (Math|Integer|Clamp(Integer) _result 0 2) 1)
          (Variables|Default|SetbCamShakeActivated true))))))

(event OnComponentBeginOverlap(Sphere)
  (params (OverlappedComponent :type Primitive%20Component%20Object%20Reference) (OtherActor :type Actor%20Object%20Reference) (OtherComp :type Primitive%20Component%20Object%20Reference) (OtherBodyIndex :type Integer) (bFromSweep :type Boolean) (SweepResult :type Hit%20Result%20Structure%20%28by%20ref%29))
  ;[1 1 1] To get boomerang
  (bind _asbp_fpscharacter (Utilities|Casting|CastToBP_FPSCharacter OtherActor))
  (Default|TakeBoomerang _asbp_fpscharacter)
  (Utilities|FlowControl|Delay 0.0)
  (Actor|DestroyActor))

(event Custom|RotateMesh
  ;[1 1 1] While moving boomerang rotates
  (Transformation|AddLocalRotation (Variables|Default|GetStaticMesh) (Variables|Default|GetDeltaRotationBoomerang) false false))

(event Custom|CallBackBoomerang
  (params (Distance :type Float%20%28single-precision%29))
  (bind _sphere (Variables|Default|GetSphere))
  (bind _staticmesh (Variables|Default|GetStaticMesh))
  (bind _returnvalue (Transformation|GetWorldLocation _sphere))
  ;[1 1 1] Return of boomerang
  (if (Variables|Default|GetbCamShakeActivated)
    (Utilities|FlowControl|DoOnce false
      (:Completed
        (if (Variables|Default|GetbCamShakeActivated)
          (bind _output_get (Variables|Default|SetPlayRate (/ 1.75e+03 Distance)))
          (Components|Timeline|SetPlayRate (Variables|Default|GetReturnTimeline) _output_get)
          (Physics|SetSimulatePhysics (Variables|Default|GetStaticMesh) false)
          (Collision|SetCollisionEnabled _staticmesh "QueryOnly")
          (Collision|SetCollisionResponsetoAllChannels _staticmesh "ECR_Overlap")
          (Collision|SetCollisionResponsetoChannel (Variables|Default|GetSphere) "ECC_WorldStatic" "ECR_Ignore")
          (Variables|Default|SetbCalled true)
          (Variables|Default|SetDeltaRotationBoomerang "0,4.500000, 0")
          (Utilities|Time|SetTimerbyFunctionName self "ReturnRotationTimerFunc" (Utilities|Time|GetWorldDeltaSeconds) true)
          (bind _zvalue (Timeline|Rise PlayFromStart)
            (:Update
              (Transformation|SetWorldLocation _sphere (Math|Vector|MakeVector (.x _returnvalue) (.y _returnvalue) (+ (.z _returnvalue) _zvalue)) false false))
            (:Finished
              (Variables|Default|SetReturnStartLocation (Transformation|GetActorLocation))
              ;;[0.2247 0.2337 1] Return Timeline
              (bind _newtrack_0 (Timeline|ReturnTimeline PlayFromStart)
                (:Update
                  (Transformation|SetWorldLocation (Variables|Default|GetSphere) (Math|Vector|Lerp(Vector) (Variables|Default|GetReturnStartLocation) (Transformation|GetActorLocation (Variables|Default|GetInstigatorPawnRef)) _newtrack_0) true false))))))))))

(event Custom|SimulatePhysicHandle
  (bind _staticmesh (Variables|Default|GetStaticMesh))
  ;[1 1 1] When boomerang hit stop timeline, clear timer, ticking disabled. Simulate physics is activated!
  (Components|Activation|Deactivate (Variables|Default|GetForward))
  (Utilities|Time|PauseTimerbyHandle (Variables|Default|GetRotateTimerHandle))
  (Actor|Tick|SetActorTickEnabled false)
  (Collision|SetCollisionResponsetoAllChannels _staticmesh "ECR_Block")
  (Collision|SetCollisionEnabled (Variables|Default|GetStaticMesh) "PhysicsOnly")
  (Collision|SetCollisionResponsetoChannel (Variables|Default|GetSphere) "ECC_Pawn" "ECR_Overlap")
  (Physics|SetSimulatePhysics _staticmesh true))

(event EventDestroyed
  (bind _asbp_fpscharacter (Utilities|Casting|CastToBP_FPSCharacter (Variables|Default|GetInstigatorPawnRef)))
  (Default|BoomerangCamShake _asbp_fpscharacter))

(event EventBeginPlay
  ;[1 1 1] To turn back character, get reference of pawn
  (bind _output_get (Variables|Default|SetInstigatorPawnRef (Game|GetInstigator)))
  (bind _asbp_fpscharacter (Utilities|Casting|CastToBP_FPSCharacter _output_get))
  (Variables|Default|SetBoomerang%20Charge (Variables|/Game/Blueprints/Character/BP_FPSCharacter.BP_FPSCharacter_C|GetBoomerangCharge _asbp_fpscharacter))
  ;[1 1 1] to prevent pawn = nullptr
  (Utilities|FlowControl|Delay 0.0)
  (Variables|Default|SetInitialPawnForwardVector (Transformation|GetActorForwardVector (Variables|Default|GetInstigatorPawnRef)))
  (Actor|Tick|SetActorTickEnabled false)
  (bind _returnvalue (Utilities|Time|SetTimerbyEvent (delegate Custom|RotateMesh) (Utilities|Time|GetWorldDeltaSeconds) true))
  (Variables|Default|SetRotateTimerHandle _returnvalue)
  (Variables|Default|SetInitialLocation (Transformation|GetActorLocation))
  ;[1 1 1] Forward Timeline Handle
  (Components|Timeline|SetPlayRate (Variables|Default|GetForward) (Variables|Default|GetTimelineRate))
  (bind _deltalocation (Timeline|Forward PlayFromStart)
    (:Update
      (Transformation|AddLocalOffset (Variables|Default|GetSphere) (* (Math|Vector|MakeVector (.x _deltalocation) (* (.y _deltalocation) (Variables|Default|GetBoomerang%20Charge)) (.z _deltalocation)) (Variables|Default|GetBoomerangRangeMultiplier)) true false))
    (:Finished
      (Utilities|Time|ClearandInvalidateTimerbyHandle (Variables|Default|GetRotateTimerHandle))
      (Variables|Default|SetbCamShakeActivated true)
      (CallFunction|SimulatePhysicHandle))
    (:DistanceCheck
      (if (<= (Math|Vector|Distance(Vector) (Transformation|GetActorLocation) (Transformation|GetActorLocation (Variables|Default|GetInstigatorPawnRef))) 2.5e+02)
        (Components|Activation|Deactivate (Variables|Default|GetForward))
        (Actor|Tick|SetActorTickEnabled true)))))

(event EventTick
  (params (DeltaSeconds :type Float%20%28single-precision%29))
  ;[1 1 1] Turn back while ticking. Initially is not ticking!
  (Transformation|SetActorLocation (Math|Interpolation|VInterpTo (Transformation|GetActorLocation) (Transformation|GetActorLocation (Variables|Default|GetInstigatorPawnRef)) DeltaSeconds 15.0) true false))

(fn ConstructionScript
  (Actor|Tick|SetActorTickEnabled false))

(fn ReturnRotationTimerFunc
  (Transformation|AddWorldRotation (Variables|Default|GetStaticMesh) (Variables|Default|GetDeltaRotationBoomerang) false false))