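; Objective manager that teleports the player to the boomerang area after the HL gun objective.
; Overlapping its box with an "Us"-tagged actor moves the overlapping component, sends a gun-drop message, and spawns a translucent wall with a camera view to protect the boomerang target.
; A looping timer then spawns enemy balls using random target points.
; DestroyTranslucentWall, called upon target destruction, removes the wall and its widget and stops the timer.
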(event OnComponentBeginOverlap(Box)
  (params (OverlappedComponent :type Primitive%20Component%20Object%20Reference) (OtherActor :type Actor%20Object%20Reference) (OtherComp :type Primitive%20Component%20Object%20Reference) (OtherBodyIndex :type Integer) (bFromSweep :type Boolean) (SweepResult :type Hit%20Result%20Structure%20%28by%20ref%29))
  (if (Actor|ActorHasTag OtherActor "Us")
    (Transformation|SetWorldLocation OtherComp (Variables|Default|GetTPLocation) false true)
    (Class|BPIInteraction|DropHLGun(Message) OtherActor) ; disable HL gun
    (bind _returnvalue (Game|SpawnActorfromClass "/Game/Blueprints/Boomerang/BoomerangTarget/BP_TranslucentWall.BP_TranslucentWall_C" (Variables|Default|GetWallTransform_0) "AlwaysSpawn" 0 0)) ; to protect boomerang target
    (bind _output_get (Variables|Default|SetWallRef _returnvalue))
    (Default|ShowCameraView _output_get) ; there is helper camere above the wall
    (bind _returnvalue_2 (Utilities|Time|SetTimerbyEvent (delegate Custom|SpawnEnemyBall) 4.0 true))
    (Variables|Default|SetSpawnEnemyBallTimer _returnvalue_2)
    (Audio|SpawnSound2D "/Engine/VREditor/Sounds/UI/Teleport_Committed.Teleport_Committed" 1.0 1.0 0.0 0)))

(event Custom|SpawnEnemyBall
  (bind _targetpoints (Variables|Default|GetTargetPoints))
  (bind _outitem (Utilities|Array|Random _targetpoints))
  (bind _arrowcomponent (Variables|/Script/Engine.TargetPoint|GetArrowComponent _outitem))
  (bind _returnvalue (Transformation|GetWorldTransform _arrowcomponent))
  (Game|SpawnActorfromClass "/Game/AI_Enemy/BP_EnemyBall.BP_EnemyBall_C" (Math|Transform|MakeTransform (.location _returnvalue) (.rotation _returnvalue) "0.400000,0.400000,0.400000") "AlwaysSpawn" 0 0)
  (Audio|SpawnSoundatLocation "/Engine/EditorSounds/GamePreview/EndSimulate.EndSimulate" (.location _returnvalue) "0, 0, 0" 1.0 1.0 0.0 0 0))

(event EventDestroyTranslucentWall
  (bind _wallref (Variables|Default|GetWallRef))
  ;[1 1 1] It's called when Boomerang Target is destroyed
  (Utilities|IsValid _wallref
    (:Is%20Valid
      (Default|RemoveWidget _wallref)
      (Actor|DestroyActor _wallref)
      (Utilities|Time|ClearandInvalidateTimerbyHandle (Variables|Default|GetSpawnEnemyBallTimer)))))

(fn ConstructionScript)

(fn OutputTry
  (params (Input :type Integer))
  (return false))