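; BP_PointManager is an objective actor that rewards the player with a BP_HLGun once three point targets have been scored.
; Point actors fire its MadeScore event, which increments PointCounter and checks it against three.
; On a match it spawns the gun at its root transform, yawed a further 90 degrees, and plays a 2D prize sound.
; The OutputTry function is a stub that always returns false.
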(event EventMadeScore
  (bind _defaultsceneroot (Variables|Default|GetDefaultSceneRoot))
  (bind _returnvalue (Transformation|GetWorldTransform _defaultsceneroot))
  (bind _result (Math|Integer|IncrementInt (Variables|Default|GetPointCounter))
    (:%20%20
      (if (== _result 3)
        (Game|SpawnActorfromClass "/Game/Blueprints/Weapons/BP_HLGun.BP_HLGun_C" (Math|Transform|MakeTransform (.location _returnvalue) (Math|Rotator|MakeRotator (.roll (.rotation _returnvalue)) (.pitch (.rotation _returnvalue)) (+ (.yaw (.rotation _returnvalue)) 9e+01)) (.scale _returnvalue)) "AlwaysSpawn" 0 0) ; if we have enough point, this node spawns HL Gun
        (Audio|SpawnSound2D "/Game/Sounds/Gameplay/prize.prize" 1.0 1.0 0.0 0)))))

(fn ConstructionScript)

(fn OutputTry
  (params (Input :type Integer))
  (return false))