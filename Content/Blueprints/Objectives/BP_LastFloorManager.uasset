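; Last-mission floor manager that throws the arriving player into the fight and starts an endless stream of enemy balls.
; A character tagged "Us" overlapping the Box is launched along world X, then the Box blocks Pawns after a short delay.
; SpawnBalls then re-calls itself after random delays, spawning BP_EnemyBall at random TargetPoints with randomized per-axis scale.
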(event OnComponentBeginOverlap(Box)
  (params (OverlappedComponent :type Primitive%20Component%20Object%20Reference) (OtherActor :type Actor%20Object%20Reference) (OtherComp :type Primitive%20Component%20Object%20Reference) (OtherBodyIndex :type Integer) (bFromSweep :type Boolean) (SweepResult :type Hit%20Result%20Structure%20%28by%20ref%29))
  ;[1 1 1] When the player arrives the last floor (last mission) this actor launches the player into the fire
  (if (Actor|ActorHasTag OtherActor "Us")
    (bind _ascharacter (Utilities|Casting|CastToCharacter OtherActor))
    (Character|LaunchCharacter _ascharacter "2000.000000, 0, 0" true false)
    (Utilities|FlowControl|Delay 0.2)
    (Collision|SetCollisionResponsetoChannel (Variables|Default|GetBox) "ECC_Pawn" "ECR_Block")
    (CallFunction|SpawnBalls)))

(event Custom|SpawnBalls
  (bind _returnvalue (Math|Random|RandomFloatinRange 0.4 1.0))
  (bind _targetpoints (Variables|Default|GetTargetPoints))
  (bind _outitem (Utilities|Array|Random _targetpoints))
  (bind _returnvalue_2 (Transformation|GetActorTransform _outitem))
  ;[1 1 1] When the player arrives the last floor (last mission) this actor starts to spawn enemy balls
  (Game|SpawnActorfromClass "/Game/AI_Enemy/BP_EnemyBall.BP_EnemyBall_C" (Math|Transform|MakeTransform (.location _returnvalue_2) (.rotation _returnvalue_2) (Math|Vector|MakeVector _returnvalue _returnvalue _returnvalue)) "AlwaysSpawn" 0 0)
  (Variables|Default|SetSpawnRate (Math|Random|RandomFloatinRange 2.5 3.5))
  (Utilities|FlowControl|Delay (Variables|Default|GetSpawnRate))
  (CallFunction|SpawnBalls))

(fn ConstructionScript)