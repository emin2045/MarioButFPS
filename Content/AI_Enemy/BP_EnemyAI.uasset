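; Enemy AI character that spawns a socketed weapon and fires it when its behavior tree calls Fire.
; First sight or first damage starts the tree and removes PawnSensing; damage also turns it toward the causer, while sight starts timed random wander through Blackboard keys.
; Zero health or BoomerangDestroyed stops the brain, ragdolls the mesh and schedules cleanup.
; BlackholeEffect switches to flying and pulls the enemy toward the origin on Tick briefly.
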(event OnSeePawn(PawnSensing)
  (params (Pawn :type Pawn%20Object%20Reference))
  ;[1 1 1] When the enemy see us, it's behavior tree starts to run and according to BT, it actions.
  (Utilities|FlowControl|DoOnce false
    (:Completed
      (bind _asbp_aicontroller (Utilities|Casting|CastToBP_AIController (AI|GetAIController self))
        (:then
          (AI|RunBehaviorTree _asbp_aicontroller "/Game/AI_Enemy/BT_Enemy.BT_Enemy")
          (bind _pawnsensing (Variables|Default|GetPawnSensing)
            (:then
              (Components|DestroyComponent _pawnsensing))
            (:else
              _))
          (AI|Components|Blackboard|SetValueasFloat (AI|GetBlackboard 0) (Utilities|Name|MakeLiteralName "WaitTime") (Variables|Default|GetWaitTime))
          (Utilities|Time|SetTimerbyEvent (delegate Custom|SetRandomLocationToGo) (Variables|Default|GetWaitTime) true))
        (:CastFailed
          (Development|PrintString "AI cast failed"))))))

(event Custom|BlackholeEffect
  (params (BlackholeOrigin :type Vector))
  ;[1 1 1] BlackholeEffect
  (Pawn|Components|CharacterMovement|SetMovementMode (Variables|Character|GetCharacterMovement) "MOVE_Flying" 0)
  (Variables|Default|SetBlackholeOrigin BlackholeOrigin)
  (Actor|Tick|SetActorTickEnabled true)
  (Variables|Default|SetbBlackholeActivated true)
  (Utilities|FlowControl|Delay 2.3)
  (Actor|Tick|SetActorTickEnabled false)
  (Pawn|Components|CharacterMovement|SetMovementMode (Variables|Character|GetCharacterMovement) "MOVE_Walking" 0))

(event Custom|Fire
  (params (TargetPawn :type Pawn%20Object%20Reference))
  ;[1 1 1] Called from Behavior Tree Fire
  (Default|AIFire (Variables|Default|GetWeaponRef) TargetPawn (Variables|Default|GetBaseDamage)))

(event Custom|SetRandomLocationToGo
  (bind _returnvalue (Math|Random|RandomUnitVector))
  (bind _returnvalue_2 (AI|GetBlackboard 0))
  ;[1 1 1] Set Random Location For AI_Enemy. It goes to that location
  (Utilities|FlowControl|FlipFlop
    (:A
      (bind _output_get (Variables|Default|SetbWantsGoAI true))
      (AI|Components|Blackboard|SetValueasVector _returnvalue_2 (Utilities|Name|MakeLiteralName "DesiredLocation") (+ (Transformation|GetActorLocation) (Math|Vector|MakeVector (* (.x _returnvalue) 3e+02) (* (.y _returnvalue) 3e+02) 0.0)))
      (AI|Components|Blackboard|SetValueasBool _returnvalue_2 (Utilities|Name|MakeLiteralName "WantsToGo") _output_get))
    (:B
      (bind _output_get_2 (Variables|Default|SetbWantsGoAI false))
      (AI|Components|Blackboard|SetValueasBool (AI|GetBlackboard 0) (Utilities|Name|MakeLiteralName "WantsToGo") _output_get_2))))

(event Custom|RotateEnemyToDamageCause
  ;[1 1 1] Damage Handle
  (Transformation|SetActorRotation (Math|Interpolation|RInterpTo (Transformation|GetActorRotation) (Math|Rotator|FindLookatRotation (Transformation|GetActorLocation) (Transformation|GetActorLocation (stale Game|Damage|EventAnyDamage DamageCauser))) (Utilities|Time|GetWorldDeltaSeconds) 8.0)))

(event Game|Damage|EventAnyDamage
  (params (Damage :type Float%20%28single-precision%29) (DamageType :type Damage%20Type%20Object%20Reference) (InstigatedBy :type Controller%20Object%20Reference) (DamageCauser :type Actor%20Object%20Reference))
  (bind _mesh (Variables|Character|GetMesh))
  ;[1 1 1] Damage Handle
  (Utilities|FlowControl|Sequence
    (:then_0
      (Utilities|FlowControl|DoOnce false
        (:Completed
          (bind _asbp_aicontroller (Utilities|Casting|CastToBP_AIController (AI|GetAIController self)))
          (AI|RunBehaviorTree _asbp_aicontroller "/Game/AI_Enemy/BT_Enemy.BT_Enemy")
          (bind _pawnsensing (Variables|Default|GetPawnSensing)
            (:then
              (Components|DestroyComponent _pawnsensing)
              (bind _returnvalue (Utilities|Time|SetTimerbyEvent (delegate Custom|RotateEnemyToDamageCause) (Utilities|Time|GetWorldDeltaSeconds) true))
              (Utilities|FlowControl|Delay 1.5)
              (Utilities|Time|ClearandInvalidateTimerbyHandle _returnvalue))
            (:else)))))
    (:then_1
      (if (> (Variables|Default|GetHealth) 0.0)
        (bind _output_get (Variables|Default|SetHealth (Math|Float|Clamp(Float) (- (Variables|Default|GetHealth) Damage) 0.0 1e+02)))
        (if (== _output_get 0.0)
          (Utilities|FlowControl|Sequence
            (:then_0
              ;;[1 1 1] 1
              (bind _braincomponent (Variables|/Script/AIModule.AIController|GetBrainComponent (AI|GetAIController self))
                (:then
                  (AI|Logic|StopLogic _braincomponent "Dead")
                  (Pawn|Components|CharacterMovement|DisableMovement (Variables|Character|GetCharacterMovement)))
                (:else
                  (Development|PrintString "AI_Enemy Brain not found")
                  ;;[1 1 1] 2
                  (Collision|SetCollisionEnabled (Variables|Character|GetMesh) "QueryAndPhysics" :!label _label)
                  (Collision|SetCollisionResponsetoChannel _mesh "ECC_WorldStatic" "ECR_Block")
                  (Class|SkeletalMeshComponent|SetAllBodiesSimulatePhysics _mesh true)
                  (Class|SkeletalMeshComponent|SetAllBodiesPhysicsBlendWeight _mesh 1.0 false))))
            (:then_1
              (goto _label))
            (:then_2
              ;;[1 1 1] 3
              (Actor|SetLifeSpan (Variables|Default|GetWeaponRef) (Variables|Default|GetDestroyActorRate))
              (Actor|SetLifeSpan (Variables|Default|GetDestroyActorRate)))))))))

(event EventTick
  (params (DeltaSeconds :type Float%20%28single-precision%29))
  ;[1 1 1] When blackhole activated set true, the blackhole impact works
  (if (Variables|Default|GetbBlackholeActivated)
    (Transformation|SetActorLocation (Math|Interpolation|VInterpTo (Transformation|GetActorLocation) (Variables|Default|GetBlackholeOrigin) DeltaSeconds (Variables|Default|GetBlackholeInterpTime)) true false)))

(event EventBeginPlay
  ;[1 1 1] Initial weapon setup
  (bind _returnvalue (Game|SpawnActorfromClass "/Game/Blueprints/Weapons/BP_Weapon.BP_Weapon_C" (Math|Transform|MakeTransform "0, 0, 0") "AlwaysSpawn" self 0))
  (bind _output_get (Variables|Default|SetWeaponRef _returnvalue))
  (Transformation|AttachComponentToComponent _output_get (Variables|Character|GetMesh) "WeaponSocket" "SnapToTarget" "SnapToTarget" "SnapToTarget" true)
  (Variables|Default|SetBlackholeInterpTime (Math|Random|RandomFloatinRange 0.5 1.0)))

(event EventBoomerangDestroyed
  (bind _mesh (Variables|Character|GetMesh))
  ;[1 1 1] Damage Handle
  (Utilities|FlowControl|Sequence
    (:then_0
      ;;[1 1 1] 1
      (bind _braincomponent (Variables|/Script/AIModule.AIController|GetBrainComponent (AI|GetAIController self))
        (:then
          (AI|Logic|StopLogic _braincomponent "Dead")
          (Pawn|Components|CharacterMovement|DisableMovement (Variables|Character|GetCharacterMovement)))
        (:else
          (Development|PrintString "AI_Enemy Brain not found")
          ;;[1 1 1] 2
          (Collision|SetCollisionEnabled (Variables|Character|GetMesh) "QueryAndPhysics" :!label _label)
          (Collision|SetCollisionResponsetoChannel _mesh "ECC_WorldStatic" "ECR_Block")
          (Class|SkeletalMeshComponent|SetAllBodiesSimulatePhysics _mesh true)
          (Class|SkeletalMeshComponent|SetAllBodiesPhysicsBlendWeight _mesh 1.0 false))))
    (:then_1
      (goto _label))
    (:then_2
      ;;[1 1 1] 3
      (Actor|SetLifeSpan (Variables|Default|GetWeaponRef) (Variables|Default|GetDestroyActorRate))
      (Actor|SetLifeSpan (Variables|Default|GetDestroyActorRate)))))

(fn ConstructionScript)

(fn OutputTry
  (params (Input :type Integer))
  (return false))