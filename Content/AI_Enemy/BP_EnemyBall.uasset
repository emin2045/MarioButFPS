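; BP_EnemyBall is a kamikaze-style enemy pawn that moves toward the player and damages them on contact.
; On BeginPlay it issues a single SimpleMoveToActor on the first player character through its AI controller.
; Overlapping an actor tagged "Us" with its sphere applies BaseDamage and destroys the ball.
; Any damage it takes reduces Health, destroying it at zero and otherwise slowing its floating movement by a fixed step.
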(event OnComponentBeginOverlap(Sphere1)
  (params (OverlappedComponent :type Primitive%20Component%20Object%20Reference) (OtherActor :type Actor%20Object%20Reference) (OtherComp :type Primitive%20Component%20Object%20Reference) (OtherBodyIndex :type Integer) (bFromSweep :type Boolean) (SweepResult :type Hit%20Result%20Structure%20%28by%20ref%29))
  ;[1 1 1] If overlap with the player, applies damage to the player and destroy itself
  (if (Actor|ActorHasTag OtherActor "Us")
    (Game|Damage|ApplyDamage OtherActor (Variables|Default|GetBaseDamage) 0 self)
    (Actor|DestroyActor)))

(event EventBeginPlay
  ;[1 1 1] Initialization- Determine a target. In this case the goal is the player
  (AI|Navigation|SimpleMovetoActor (AI|GetAIController self) (Game|GetPlayerCharacter 0)))

(event Game|Damage|EventAnyDamage
  (params (Damage :type Float%20%28single-precision%29) (DamageType :type Damage%20Type%20Object%20Reference) (InstigatedBy :type Controller%20Object%20Reference) (DamageCauser :type Actor%20Object%20Reference))
  (bind _floatingpawnmovement (Variables|Default|GetFloatingPawnMovement))
  ;[1 1 1] If this actor takes any damage, health and speed are ddecreased
  (bind _output_get (Variables|Default|SetHealth (- (Variables|Default|GetHealth) Damage)))
  (if (<= _output_get 0.0)
    (Actor|DestroyActor)
    (else
      (Variables|/Script/Engine.FloatingPawnMovement|SetMaxSpeed _floatingpawnmovement (- (Variables|/Script/Engine.FloatingPawnMovement|GetMaxSpeed _floatingpawnmovement) 8e+01)))))

(fn ConstructionScript)